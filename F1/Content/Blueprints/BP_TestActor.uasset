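; BP_TestActor is a test actor that exercises array iteration, text formatting and a simple function call by printing the results.
; On BeginPlay it loops over the Level array and prints each element with its index through FormatText.
; Every Tick it calls TestFunc, which adds two inputs, with constant arguments and prints the sum.
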(event `self.ReceiveBeginPlay`
  (for (_array_element _array_index) (`self.Level`)
    (`KismetSystemLibrary.PrintText` (`|FormatText` "{index} : {Element} " _array_index _array_element))))

(event `self.ReceiveTick`
  (params (DeltaSeconds :type "Float (single-precision)"))
  (bind _returnvalue (`self.TestFunc` 10 20))
  (`KismetSystemLibrary.PrintString` (`KismetStringLibrary.Conv_IntToString` _returnvalue)))

(fn `TestFunc`
  (params (A :type Integer) (B :type Integer))
  (returns (ReturnValue :type Integer))
  (return (+ A B)))

(fn `UserConstructionScript`)